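; Player character for the Runner, which moves, looks around, collects keys and triggers traps.
; Axis inputs drive controller look and yaw-relative movement, and possession by a player controller hides the mouse cursor.
; Key overlaps add their value to the play-mode game state's money, while trap overlaps set the interactable that the interact input enables if not already enabled.
; GetName returns the player name stored in the game instance.
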(event Collision|EventActorBeginOverlap
  (params (OtherActor :type Actor%20Object%20Reference))
  ;[1 1 1] Add money
  (bind _asbp_key (Utilities|Casting|CastToBP_Key OtherActor)
    (:then
      (Default|AddMoney (.AsGS%20Play%20Mode (Utilities|Casting|CastToGS_PlayMode (Game|GetGameState))) (Variables|/Game/Blueprints/Actors/BP_Key.BP_Key_C|GetValue _asbp_key)))
    (:CastFailed
      (bind _asbp_trap (Utilities|Casting|CastToBP_Trap OtherActor))
      (Variables|Components|SetInteractable _asbp_trap))))

(event Collision|EventActorEndOverlap
  (params (OtherActor :type Actor%20Object%20Reference))
  ;[1 1 1] Add money
  (Utilities|Casting|CastToBP_Trap OtherActor)
  (Variables|Components|SetInteractable 0))

(event EventPossessed
  (params (NewController :type Controller%20Object%20Reference))
  ;[1 1 1] Hides the cursor of the player
  (bind _asplayer_controller (Utilities|Casting|CastToPlayerController NewController))
  (Variables|/Script/Engine.PlayerController|SetbShowMouseCursor _asplayer_controller false))

(event Input|ActionEvents|InputActionInputRunner_Interact
  (params (Key :type Key%20Structure))
  (bind _interactable (Variables|Components|GetInteractable))
  ;[1 1 1] Traps interaction
  (:Pressed
    (Utilities|IsValid _interactable
      (:Is%20Valid
        (if (not (Variables|/Game/Blueprints/Actors/BP_Trap.BP_Trap_C|GetIsEnabled _interactable))
          (Default|Enable _interactable))))))

(event Input|AxisEvents|InputAxisLook_Axis_Y
  (params (AxisValue :type Float%20%28single-precision%29))
  ;[1 1 1] Camera
  (Pawn|Input|AddControllerPitchInput AxisValue))

(event Input|AxisEvents|InputAxisLook_Axis_X
  (params (AxisValue :type Float%20%28single-precision%29))
  ;[1 1 1] Camera
  (Pawn|Input|AddControllerYawInput AxisValue))

(event Input|AxisEvents|InputAxisMove_Forward
  (params (AxisValue :type Float%20%28single-precision%29))
  ;[1 1 1] Movement
  (Pawn|Input|AddMovementInput (Math|Vector|GetForwardVector (Math|Rotator|MakeRotator 0.0 0.0 (.yaw (Pawn|GetControlRotation :!class /Script/Engine.Pawn)))) AxisValue false)
  (if (> (Math|Vector|VectorLength (Transformation|GetVelocity)) 0.0)
    _))

(event Input|AxisEvents|InputAxisMove_Strafe
  (params (AxisValue :type Float%20%28single-precision%29))
  ;[1 1 1] Movement
  (Pawn|Input|AddMovementInput (Math|Vector|GetRightVector (Math|Rotator|MakeRotator 0.0 0.0 (.yaw (Pawn|GetControlRotation :!class /Script/Engine.Pawn)))) AxisValue false)
  (if (> (Math|Vector|VectorLength (Transformation|GetVelocity)) 0.0)
    _))

(fn ConstructionScript)

(fn GetName
  (return (Utilities|Text|ToText(Name) (.name (Variables|/Game/Blueprints/GameInstances/GI_GameInstanceInfos.GI_GameInstanceInfos_C|GetM%20PlayerInfos (.AsGI%20Game%20Instance%20Infos (Utilities|Casting|CastToGI_GameInstanceInfos (Game|GetGameInstance))))))))