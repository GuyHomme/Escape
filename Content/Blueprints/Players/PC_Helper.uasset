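; Player controller for a helper role that clicks in the world to buy doors open or place lights for a second player.
; Cursor traces open doors for Money, branching on authority, with the map legend sprite swapped only on the authority path; other hits spawn BP_Lumos and notify GS_PlayMode, gated by a cooldown.
; Tick counts down that cooldown and keeps the second player's name actor following them; O triggers server travel.
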(event Custom|SpawnLight
  (params (Location :type Vector))
  (bind (_x _y _z) (Math|Vector|BreakVector Location))
  ;[1 1 1] Lights
  (Game|SpawnActorfromClass "/Game/Blueprints/Actors/BP_Lumos.BP_Lumos_C" (Math|Transform|MakeTransform (Math|Vector|MakeVector _x _y (+ _z 1e+02)) "0, 0, 0" "1,1,1") "Undefined" 0 0)
  (Default|Lumos (.AsGS%20Play%20Mode (Utilities|Casting|CastToGS_PlayMode (Game|GetGameState)))))

(event Custom|SpawnLightAsClient
  (params (Location :type Vector))
  ;[1 1 1] Lights
  (CallFunction|SpawnLight Location))

(event Custom|OpenAsClient
  (params (Door :type BP%20Door%20Object%20Reference))
  ;[1 1 1] Clicking
  (Default|OpenDoor Door))

(event EventTick
  (params (DeltaSeconds :type Float%20%28single-precision%29))
  ;[1 1 1] Lights cooldown
  (Utilities|FlowControl|Sequence
    (:then_0
      (if (Variables|Components|GetLightInCD)
        (Variables|Components|SetCooldDown (- (Variables|Components|GetCooldDown) DeltaSeconds))
        (bind _return (CallFunction|CanSpawnLight))
        (if _return
          (Variables|Components|SetLightInCD false))))
    (:then_1
      (if (Variables|References|GetGameStarted)
        (CallFunction|UpdateSndPlayerName)))))

(event Input|MouseEvents|LeftMouseButton
  (params (Key :type Key%20Structure))
  (bind _returnvalue (Game|GetPlayerController 0))
  (bind _hitresult (Game|Player|GetHitResultUnderCursorbyChannel _returnvalue "TraceTypeQuery1" true))
  (bind (_bblockinghit _binitialoverlap _time _distance _location _impactpoint _normal _impactnormal _physmat _hitactor) (Collision|BreakHitResult _hitresult))
  ;[1 1 1] Clicking
  (:Pressed
    (if _bblockinghit
      (bind _asbp_door (Utilities|Casting|CastToBP_Door _hitactor)
        (:then
          (if (not (Variables|/Game/Blueprints/Actors/BP_Door.BP_Door_C|GetIsOpened _asbp_door))
            (if (>= (Variables|Components|GetMoney) (Variables|/Game/Blueprints/Actors/BP_Door.BP_Door_C|GetCost _asbp_door))
              (CallFunction|RemoveMoney (Variables|/Game/Blueprints/Actors/BP_Door.BP_Door_C|GetCost _asbp_door))
              (Networking|SwitchHasAuthority
                (:Authority
                  (Default|OpenDoor _asbp_door)
                  (Rendering|Components|Sprite|SetSprite (Utilities|Array|Get(acopy) (Actor|GetComponentsbyTag _asbp_door "/Script/Paper2D.PaperSpriteComponent" "MapLegend")) "/Game/Sprites/30776631_10213952554802034_1255386392_n_Sprite.30776631_10213952554802034_1255386392_n_Sprite"))
                (:Remote
                  (CallFunction|OpenasClient _asbp_door))))))
        (:CastFailed
          (bind _return (CallFunction|CanSpawnLight))
          (if _return
            (Variables|Components|SetLightInCD true)
            (Variables|Components|SetCooldDown (Utilities|CONSTLightCooldown))
            (CallFunction|SpawnLightasClient _location)))))))

(event Input|KeyboardEvents|O
  (params (Key :type Key%20Structure))
  (:Pressed
    (Default|ServerTravel (.AsGI%20Game%20Instance%20Infos (Utilities|Casting|CastToGI_GameInstanceInfos (Game|GetGameInstance))))))

(fn ConstructionScript)

(fn AddMoney
  (params (Money :type Integer))
  (Variables|Components|SetMoney (+ Money (Variables|Components|GetMoney))))

(fn RemoveMoney
  (params (Amount :type Integer))
  (Variables|Components|SetMoney (- (Variables|Components|GetMoney) Amount)))

(fn CanSpawnLight
  (return (<= (Variables|Components|GetCooldDown) 0.0)))

(fn UpdateSndPlayerName
  (bind _sndplayerref (Variables|References|GetSndPlayerRef))
  (bind _returnvalue (Transformation|GetActorLocation _sndplayerref))
  (if (Variables|/Game/Blueprints/PlayerStates/PS_PlayInfos.PS_PlayInfos_C|GetStillUp (.AsPS%20Play%20Infos (Utilities|Casting|CastToPS_PlayInfos (Variables|GetPlayerState))))
    (Transformation|SetActorLocation (Variables|References|GetSndPlayerNameRef) (Math|Vector|MakeVector (.x _returnvalue) (.y _returnvalue) 0.0) false false)))