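; HUD Blueprint for play that shows the role choice screen, where the player picks a role such as Runner or Helper.
; On BeginPlay it adds a copyright widget and a role choice widget to the viewport.
; Events store the acquired role in the player's PS_PlayInfos PlayerState, hide a given role in the widget, or remove the choice widget.
; A helper function maps each role to its opposite.
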(event Custom|RoleAcquired
  (params (Role :type PlayerRole%20Enum :default "NewEnumerator2"))
  ;[1 1 1] Setting of the role chosen by player
  (Default|SetRole (.AsPS%20Play%20Infos (Utilities|Casting|CastToPS_PlayInfos (Variables|/Script/Engine.Controller|GetPlayerState (Game|GetPlayerController 0)))) Role))

(event Custom|ClearHUD
  ;[1 1 1] Setting of the role chosen by player
  (Widget|RemovefromParent (Variables|References|GetWBP_RoleChoice)))

(event Custom|MyWork
  ;[1 1 1] Copyright
  (bind _returnvalue (UserInterface|CreateWidget "/Game/Blueprints/Widgets/WBP_Copyright.WBP_Copyright_C" (Game|GetPlayerController 0)))
  (UserInterface|Viewport|AddtoViewport _returnvalue 0))

(event Custom|HideThisRole
  (params (Role :type PlayerRole%20Enum :default "NewEnumerator2"))
  ;[1 1 1] Setting of the role chosen by player
  (Default|HideRole (Variables|References|GetWBP_RoleChoice) Role))

(event EventBeginPlay
  ;[1 1 1] Choice widget addition
  (CallFunction|MyWork)
  (Utilities|IsValid (Variables|References|GetWBP_RoleChoice)
    (:Is%20Valid
      _)
    (:Is%20Not%20Valid
      (bind _returnvalue (UserInterface|CreateWidget "/Game/Blueprints/Widgets/WBP_RoleChoice.WBP_RoleChoice_C" (Game|GetPlayerController 0)))
      (bind _output_get (Variables|References|SetWBP_RoleChoice _returnvalue))))
  (UserInterface|Viewport|AddtoViewport _output_get 0))

(fn ConstructionScript)

(fn ReversedRole
  (params (InRole :type PlayerRole%20Enum :default "NewEnumerator2"))
  (switch Utilities|FlowControl|Switch|SwitchonPlayerRole InRole
    (:NewEnumerator2
      (return "NewEnumerator2"))
    (:NewEnumerator0
      (return "NewEnumerator1"))
    (:NewEnumerator1
      (return "NewEnumerator0"))))