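; Game instance that holds the local player's info and manages main menu, lobby menu and multiplayer session flow.
; Player info is refreshed from the lobby PlayerState, with a separate event to set the role.
; Hosting and joining use console open commands, then share a delayed step that caches the lobby GameState and shows the lobby widget.
; Starting the game and losing both issue a servertravel to the runner level.
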(event Custom|EnterLobby
  ;[1 1 1] Enters lobby by adding a new player and calling display lobby menu
  (Utilities|IsValid (Variables|References|GetM%20LobbyMenuRef)
    (:Is%20Valid
      _)
    (:Is%20Not%20Valid
      (bind _returnvalue (UserInterface|CreateWidget "/Game/Blueprints/Widgets/WBP_LobbyMenu.WBP_LobbyMenu_C"))
      (Variables|References|SetM%20LobbyMenuRef _returnvalue)))
  (CallFunction|DisplayLobbyMenu true))

(event Custom|DisplayLobbyMenu
  (params (Show :type Boolean))
  ;[1 1 1] Displays Lobby menu
  (if Show
    (UserInterface|Viewport|AddtoViewport (Variables|References|GetM%20LobbyMenuRef) 0)
    (Default|DisplayPlayers (Variables|References|GetM%20LobbyMenuRef))
    (else
      (Widget|RemovefromParent (Variables|References|GetM%20LobbyMenuRef)))))

(event Custom|SetRole
  (params (Role :type PlayerRole%20Enum :default "NewEnumerator2"))
  (Variables|PlayerInfos|SetM%20PlayerInfos (Utilities|Struct|MakePlayerInfos (.name (Variables|PlayerInfos|GetM%20PlayerInfos)) (.image (Variables|PlayerInfos|GetM%20PlayerInfos)) Role (.id (Variables|PlayerInfos|GetM%20PlayerInfos)))))

(event Custom|Lose
  ;[1 1 1] Restart
  (Development|ExecuteConsoleCommand (Utilities|String|Append "servertravel " "Level_Runner")))

(event Custom|JoinServer
  (params (IP :type String))
  ;[1 1 1] Creates / Joins server
  ;;[0.972 1 0.9519] Joins server
  (Development|ExecuteConsoleCommand (Utilities|String|Append "open " IP))
  (Utilities|FlowControl|Delay 1.0)
  (bind _asgs_lobby (Utilities|Casting|CastToGS_Lobby (Game|GetGameState)))
  (Variables|References|SetM%20GameStateRef _asgs_lobby)
  (CallFunction|EnterLobby))

(event Custom|ServerTravel
  ;[1 1 1] Changes the map
  (Development|ExecuteConsoleCommand (Utilities|String|Append "servertravel " "Level_Runner")))

(event Custom|CreateServer
  ;[1 1 1] Creates / Joins server
  ;;[1 1 1] Create server and move to Lobby_Level
  (Development|ExecuteConsoleCommand "open Level_Lobby?listen")
  (Utilities|FlowControl|Delay 1.0)
  (bind _asgs_lobby (Utilities|Casting|CastToGS_Lobby (Game|GetGameState)))
  (Variables|References|SetM%20GameStateRef _asgs_lobby)
  (CallFunction|EnterLobby))

(event Custom|RefreshInfosFromPlayerState
  (Variables|PlayerInfos|SetM%20PlayerInfos (Variables|/Game/Blueprints/PlayerStates/PS_LobbyInfos.PS_LobbyInfos_C|GetM%20PlayerInfos (.AsPS%20Lobby%20Infos (Utilities|Casting|CastToPS_LobbyInfos (Variables|/Script/Engine.Controller|GetPlayerState (Game|GetPlayerController 0)))))))

(event Custom|DisplayMainMenu
  (params (Show :type Boolean))
  ;[1 1 1] Displays Main menu
  (if Show
    (bind _returnvalue (UserInterface|CreateWidget "/Game/Blueprints/Widgets/WBP_MainMenu.WBP_MainMenu_C"))
    (bind _output_get (Variables|References|SetM%20MainMenuWidget _returnvalue))
    (UserInterface|Viewport|AddtoViewport _output_get 0)
    (else
      (Widget|RemovefromParent (Variables|References|GetM%20MainMenuWidget)))))