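; BP_Killer is an AI chaser character that hunts the PC_Runner and triggers the game loss on capsule contact.
; Tick drives a delayed re-path toward the first runner found once GameStarted is set, plus a slow timer restoring base speed after SlowDown.
; A detection trigger gates proximity audio playback.
; Hits call Lose on game state and game instance, directly with authority or through LoseRemote otherwise.
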(event OnComponentBeginOverlap(DetectionTrigger)
  (params (OverlappedComponent :type Primitive%20Component%20Object%20Reference) (OtherActor :type Actor%20Object%20Reference) (OtherComp :type Primitive%20Component%20Object%20Reference) (OtherBodyIndex :type Integer) (bFromSweep :type Boolean) (SweepResult :type Hit%20Result%20Structure%20%28by%20ref%29))
  ;[1 1 1] Sounds
  (Utilities|Casting|CastToPC_Runner OtherActor)
  (Utilities|FlowControl|Gate true) ; enters at Open
)

(event OnComponentEndOverlap(DetectionTrigger)
  (params (OverlappedComponent :type Primitive%20Component%20Object%20Reference) (OtherActor :type Actor%20Object%20Reference) (OtherComp :type Primitive%20Component%20Object%20Reference) (OtherBodyIndex :type Integer))
  ;[1 1 1] Sounds
  (Utilities|Casting|CastToPC_Runner OtherActor)
  (Utilities|FlowControl|Gate true) ; enters at Close
)

(event OnComponentHit(CapsuleComponent)
  (params (HitComponent :type Primitive%20Component%20Object%20Reference) (OtherActor :type Actor%20Object%20Reference) (OtherComp :type Primitive%20Component%20Object%20Reference) (NormalImpulse :type Vector :default "0, 0, 0") (Hit :type Hit%20Result%20Structure%20%28by%20ref%29))
  (Utilities|Casting|CastToPC_Runner OtherActor)
  (Networking|SwitchHasAuthority
    (:Authority
      (Default|Lose (.AsGS%20Play%20Mode (Utilities|Casting|CastToGS_PlayMode (Game|GetGameState))))
      (Default|Lose (.AsGI%20Game%20Instance%20Infos (Utilities|Casting|CastToGI_GameInstanceInfos (Game|GetGameInstance)))))
    (:Remote
      (CallFunction|LoseRemote))))

(event Custom|SlowDown
  (params (Force :type Float%20%28single-precision%29) (SlowDuration :type Float%20%28single-precision%29))
  (bind _charactermovement (Variables|Character|GetCharacterMovement))
  ;[1 1 1] Slowing
  (Variables|Components|SetIsSlowed true)
  (Variables|/Script/Engine.CharacterMovementComponent|SetMaxWalkSpeed _charactermovement (- (Variables|/Script/Engine.CharacterMovementComponent|GetMaxWalkSpeed _charactermovement) Force))
  (Variables|Components|SetCurrentSlowDuration SlowDuration))

(event Custom|ChaseRunner
  ;[1 1 1] Pathfinding
  (bind _outactors (Actor|GetAllActorsOfClass "/Game/Blueprints/Players/PC_Runner.PC_Runner_C"))
  (Variables|Components|SetTarget (Utilities|Array|Get(acopy) _outactors))
  (AI|Navigation|SimpleMovetoActor (Pawn|GetController) (Variables|Components|GetTarget)))

(event Custom|LoseRemote
  (Default|Lose (.AsGS%20Play%20Mode (Utilities|Casting|CastToGS_PlayMode (Game|GetGameState))))
  (Default|Lose (.AsGI%20Game%20Instance%20Infos (Utilities|Casting|CastToGI_GameInstanceInfos (Game|GetGameInstance)))))

(event EventTick
  (params (DeltaSeconds :type Float%20%28single-precision%29))
  (Utilities|FlowControl|Sequence
    (:then_0
      ;[1 1 1] Slowing
      (if (Variables|Components|GetIsSlowed)
        (bind _output_get (Variables|Components|SetCurrentSlowDuration (- (Variables|Components|GetCurrentSlowDuration) DeltaSeconds)))
        (if (<= _output_get 0.0)
          (Variables|Components|SetIsSlowed false)
          (Variables|/Script/Engine.CharacterMovementComponent|SetMaxWalkSpeed (Variables|Character|GetCharacterMovement) (Variables|Components|GetBaseSpeed)))))
    (:then_1
      ;[1 1 1] Pathfinding
      (Utilities|FlowControl|Delay 2.0)
      (if (Variables|Components|GetGameStarted)
        (CallFunction|ChaseRunner)))
    (:then_2
      ;[1 1 1] Sounds
      (Utilities|FlowControl|Gate true
        (:Exit
          (if (not (Audio|Components|Audio|IsPlaying (Variables|Default|GetChannel_Event)))
            (Audio|Components|Audio|Play (Variables|Default|GetChannel_Event) 0.0)))))))

(fn ConstructionScript
  (Variables|Components|SetBaseSpeed (Variables|/Script/Engine.CharacterMovementComponent|GetMaxWalkSpeed (Variables|Character|GetCharacterMovement))))