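; BP_Trap is a toggleable trap actor that slows the killer (Jack) who enters its scalable trigger.
; While enabled, overlap with the killer's "Collider" component calls SlowJack on the first player's PlayerState.
; Separate Trapped events apply the slow, disable the trap, spawn particles and play fading audio.
; Enable and Disable raise or lower the mesh by timeline and create red or green dynamic materials.
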(event OnComponentBeginOverlap(Trigger)
  (params (OverlappedComponent :type Primitive%20Component%20Object%20Reference) (OtherActor :type Actor%20Object%20Reference) (OtherComp :type Primitive%20Component%20Object%20Reference) (OtherBodyIndex :type Integer) (bFromSweep :type Boolean) (SweepResult :type Hit%20Result%20Structure%20%28by%20ref%29))
  ;[1 1 1] Overlapping
  (if (Variables|Components|GetIsEnabled)
    (Utilities|Casting|CastToBP_Killer OtherActor)
    (if (Components|ComponentHasTag OtherComp "Collider")
      (Default|SlowJack (.AsPS%20Play%20Infos (Utilities|Casting|CastToPS_PlayInfos (Variables|/Script/Engine.Controller|GetPlayerState (Game|GetPlayerController 0)))) (Variables|Parameters|GetForce) (Variables|Parameters|GetSlowDuration)))))

(event Custom|Enable
  ;[1 1 1] Enabling and disabling
  (Variables|Components|SetIsEnabled true)
  (bind _returnvalue (Rendering|Material|CreateDynamicMaterialInstance (Rendering|Material|GetMaterial (Variables|Default|GetTrap) 0) :!class /Script/Engine.KismetMaterialLibrary))
  (Rendering|Material|SetVectorParameterValue _returnvalue "Colored" (Utilities|Struct|MakeLinearColor 255.0 0.0 0.0 1.0) :!class /Script/Engine.MaterialInstanceDynamic)
  (Audio|Components|Audio|Play (Variables|Default|GetChannel_Main) 0.0)
  (bind _lifting (Timeline|TrapAnimation PlayFromStart)
    (:Update
      (Transformation|SetRelativeLocation (Variables|Default|GetTrap) (Math|Vector|MakeVector 0.0 0.0 (Math|Float|Lerp 0.0 (Utilities|CONSTZTrapDestination) _lifting)) false false))))

(event Custom|Disable
  ;[1 1 1] Enabling and disabling
  (Variables|Components|SetIsEnabled false)
  (bind _returnvalue (Rendering|Material|CreateDynamicMaterialInstance (Rendering|Material|GetMaterial (Variables|Default|GetTrap) 0) :!class /Script/Engine.KismetMaterialLibrary))
  (Rendering|Material|SetVectorParameterValue _returnvalue "Colored" (Utilities|Struct|MakeLinearColor 0.0 255.0 0.0 1.0) :!class /Script/Engine.MaterialInstanceDynamic)
  (bind _lifting (Timeline|TrapAnimation ReverseFromEnd)
    (:Update
      (Transformation|SetRelativeLocation (Variables|Default|GetTrap) (Math|Vector|MakeVector 0.0 0.0 (Math|Float|Lerp 0.0 (Utilities|CONSTZTrapDestination) _lifting)) false false))))

(event Custom|TrappedAsClient
  (params (Jack :type BP%20Killer%20Object%20Reference))
  ;[1 1 1] Killer interactions
  (CallFunction|Trapped Jack))

(event Custom|Trapped
  (params (Jack :type BP%20Killer%20Object%20Reference))
  (bind _channel_main (Variables|Default|GetChannel_Main))
  ;[1 1 1] Killer interactions
  (Default|SlowDown Jack (Variables|Parameters|GetForce) (Variables|Parameters|GetSlowDuration))
  (CallFunction|Disable)
  (Game|SpawnActorfromClass "/Game/Blueprints/FX/BP_Particles.BP_Particles_C" (Transformation|GetActorTransform) "Undefined" 0 0)
  (Audio|Components|Audio|Play _channel_main 0.0)
  (Audio|Components|Audio|FadeOut _channel_main 3.0 0.0 :!class /Script/Engine.AudioComponent))

(fn ConstructionScript
  (bind _triggerscale (Variables|Parameters|GetTriggerScale))
  (Transformation|SetWorldScale3D (Variables|Default|GetTrigger) (Math|Vector|MakeVector _triggerscale _triggerscale _triggerscale)))