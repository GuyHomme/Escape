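; Game state for the play level of a Runner and Helper game in which the killer Jack chases the Runner.
; Role setup hides taken roles from other players, possesses the matching pawn and starts the chase once all players are ready.
; Money changes route through the server to every player state.
; It also relays slowdowns to Jack, plays ambience and effect sounds, and handles victory travel and loss.
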(event Custom|AddMoney
  (params (Money :type Integer))
  ;[1 1 1] Transactions
  (Networking|SwitchHasAuthority
    (:Authority
      (CallFunction|MoneyfromServer Money))
    (:Remote
      (CallFunction|MoneyfromClient Money))))

(event Custom|SlowDownJack
  (params (Force :type Float%20%28single-precision%29) (Duration :type Float%20%28single-precision%29))
  ;[1 1 1] Slowing down Jack
  (Default|SlowDown (Variables|References|GetJack) Force Duration))

(event Custom|MoneyFromServer
  (params (Money :type Integer))
  ;[1 1 1] Transactions
  (for _array_element (Variables|Default|GetPlayerArray)
    (bind _asps_play_infos (Utilities|Casting|CastToPS_PlayInfos _array_element))
    (Default|AddMoney _asps_play_infos Money)))

(event Custom|InitializeRoleServ
  (params (Role :type PlayerRole%20Enum :default "NewEnumerator2") (Player :type Player%20Controller%20Object%20Reference))
  (bind _playerstate (Variables|/Script/Engine.Controller|GetPlayerState Player))
  (bind _asps_play_infos (Utilities|Casting|CastToPS_PlayInfos _playerstate))
  ;[1 1 1] Initializes roles - Pawn possession
  ;;[1 0.004104 0] WATCH THIS
  (for _array_element (Variables|Default|GetPlayerArray)
    (if (not (== _array_element (Variables|/Script/Engine.Controller|GetPlayerState Player)))
      (Default|HideThisRole (.AsPS%20Play%20Infos (Utilities|Casting|CastToPS_PlayInfos _array_element)) Role)))
  (Math|Integer|IncrementInt (Variables|Components|GetReadies)
    (:%20%20
      (switch Utilities|FlowControl|Switch|SwitchonPlayerRole Role
        (:NewEnumerator0
          (bind _outactors (Actor|GetAllActorsOfClass "/Game/Blueprints/Players/PC_Runner.PC_Runner_C"))
          (Utilities|IsValid (Utilities|Array|Get(acopy) _outactors)
            (:Is%20Valid
              (Pawn|Possess Player (Utilities|Array|Get(acopy) _outactors))
              (Variables|References|SetRunner _asps_play_infos)
              (Variables|/Script/Engine.PlayerController|SetbShowMouseCursor Player false))))
        (:NewEnumerator1
          (bind _outactors_2 (Actor|GetAllActorsOfClass "/Game/Blueprints/Players/PC_Helper.PC_Helper_C"))
          (Utilities|IsValid (Utilities|Array|Get(acopy) _outactors_2)
            (:Is%20Valid
              (Pawn|Possess Player (Utilities|Array|Get(acopy) _outactors_2))
              (Variables|References|SetHelper _asps_play_infos)
              (Variables|/Script/Engine.PlayerController|SetbShowMouseCursor Player true)))))
      (Class|WidgetBlueprintLibrary|SetFocustoGameViewport)
      (if (== (Variables|Components|GetReadies) (Utilities|CONSTNbMaxPlayers))
        (Default|ReadiesOP (Variables|References|GetHelper))
        (Default|Helper (Variables|References|GetHelper))
        (Default|ReadiesOP (Variables|References|GetRunner))
        (Default|Runner (Variables|References|GetRunner))
        (CallFunction|Start)))))

(event Custom|MoneyFromClient
  (params (Money :type Integer))
  ;[1 1 1] Transactions
  (CallFunction|MoneyfromServer Money))

(event Custom|Sounds
  (bind _channel_main (Variables|Default|GetChannel_Main))
  ;[1 1 1] Sounds
  (Audio|Components|Audio|SetSound _channel_main "/Game/Audio/AmbienceSound_Creepy.AmbienceSound_Creepy")
  (Audio|Components|Audio|Play _channel_main 0.0))

(event Custom|Victory
  ;[1 1 1] End game
  (Development|ExecuteConsoleCommand (Utilities|String|Append "servertravel " "Level_Victory")))

(event Custom|Lose
  ;[1 1 1] End game
  (for _array_element (Variables|Default|GetPlayerArray)
    (Variables|/Game/Blueprints/PlayerStates/PS_PlayInfos.PS_PlayInfos_C|SetStillUp (.AsPS%20Play%20Infos (Utilities|Casting|CastToPS_PlayInfos _array_element)) false)))

(event Custom|Lumos
  (bind _channel_event (Variables|Default|GetChannel_Event))
  ;[1 1 1] Sounds
  (Audio|Components|Audio|SetSound _channel_event "/Game/Audio/SoundEffect_HarryPotter_Lumos.SoundEffect_HarryPotter_Lumos")
  (Audio|Components|Audio|Play _channel_event 0.0))

(event EventBeginPlay
  (CallFunction|Sounds))

(fn ConstructionScript)

(fn Start
  (bind _outactors (Actor|GetAllActorsOfClass "/Game/Blueprints/Actors/BP_Killer.BP_Killer_C"))
  (bind _output_get (Variables|References|SetJack (Utilities|Array|Get(acopy) _outactors)))
  (Variables|/Game/Blueprints/Actors/BP_Killer.BP_Killer_C|SetGameStarted _output_get true)
  (Default|ChaseRunner _output_get)
  (bind _outactors_2 (Actor|GetAllActorsOfClass "/Script/Engine.PlayerController"))
  (for _array_element _outactors_2
    (Utilities|Casting|CastToPC_Runner (Pawn|GetControlledPawn _array_element))
    (Variables|/Script/Engine.PlayerController|SetbShowMouseCursor _array_element false)))