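; Lobby game state that counts ready players and starts server travel once everyone is ready.
; CallReady increments MNbReady up to MaxPlayers, then loops PlayerArray and calls ServerTravel on GI_GameInstanceInfos for each entry with authority.
; An AllReady helper checks each PS_LobbyInfos MReady flag but is unused in the event graph; the MaxPlayers graph shows no body.
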(event Custom|CallReady
  (bind _nbmaxplayers (Utilities|MaxPlayers))
  (bind _m_nbready (Variables|Players|GetM%20NbReady))
  (if (< _m_nbready _nbmaxplayers)
    (bind _result (Math|Integer|IncrementInt _m_nbready)
      (:%20%20
        (if (== _result _nbmaxplayers)
          (for _array_element (Variables|Default|GetPlayerArray)
            (if (Ability|HasAuthority _array_element)
              (Default|ServerTravel (.AsGI%20Game%20Instance%20Infos (Utilities|Casting|CastToGI_GameInstanceInfos (Game|GetGameInstance)))))))))))

(fn ConstructionScript)